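; Spline generator Blueprint in the FluidNinjaLive river and landscape use case that tiles a static mesh along a spline.
; The construction script derives section length from actor scale on the forward axis and a size adjustment, then adds one spline mesh component per whole section.
; Section tangents are clamped to section length, and a valid editor placeholder material overrides the first material slot.
; It has no runtime logic.
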(event EventBeginPlay)

(event Collision|EventActorBeginOverlap
  (params (OtherActor :type Actor%20Object%20Reference)))

(event EventTick
  (params (DeltaSeconds :type Float%20%28single-precision%29)))

(fn ConstructionScript
  (bind _returnvalue (Transformation|GetActorScale3D))
  (bind _editorplaceholdermaterial (Variables|SplineGenerator|GetEditorPlaceholderMaterial))
  (bind _spline (Variables|Default|GetSpline))
  (Variables|SplineGenerator|SetSectionLength (* (Utilities|Select :Index (Variables|SplineGenerator|GetIn%20Forward%20Axis) :X (.x _returnvalue) :Y (.y _returnvalue) :Z (.z _returnvalue)) (* (Variables|SplineGenerator|GetSizeAdjutment) 1e+02)))
  (for _index (range 0 (- (Math|Float|Truncate (/ (Spline|GetSplineLength (Variables|Default|GetSpline)) (Variables|SplineGenerator|GetSectionLength))) 1))
    (bind _returnvalue_2 (AddComponent|AddSplineMeshComponent false))
    (SplineMesh|SetForwardAxis _returnvalue_2 (Variables|SplineGenerator|GetIn%20Forward%20Axis) true)
    (SplineMesh|SetStartandEnd _returnvalue_2 (Spline|GetLocationatDistanceAlongSpline _spline (* _index (Variables|SplineGenerator|GetSectionLength)) "Local") (Math|Vector|ClampVectorSize (Spline|GetTangentatDistanceAlongSpline _spline (* _index (Variables|SplineGenerator|GetSectionLength)) "Local") 0.0 (Variables|SplineGenerator|GetSectionLength)) (Spline|GetLocationatDistanceAlongSpline _spline (* (+ _index 1) (Variables|SplineGenerator|GetSectionLength)) "Local") (Math|Vector|ClampVectorSize (Spline|GetTangentatDistanceAlongSpline _spline (* (+ _index 1) (Variables|SplineGenerator|GetSectionLength)) "Local") 0.0 (Variables|SplineGenerator|GetSectionLength)) true :!class /Script/Engine.SplineMeshComponent)
    (Components|StaticMesh|SetStaticMesh _returnvalue_2 (Variables|SplineGenerator|GetStaticMeshComponent))
    (Utilities|IsValid _editorplaceholdermaterial
      (:Is%20Valid
        (Rendering|Material|SetMaterial _returnvalue_2 0 _editorplaceholdermaterial)))))